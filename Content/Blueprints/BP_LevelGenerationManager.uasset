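; Level generation manager that builds a staggered grid of hex grass tiles and scrolls it along -X like a treadmill.
; SpawnTileSet spawns static mesh actors beyond the highest cached X, starting with the initial field on BeginPlay.
; MoveTileSet adds a new set and re-caches every tile's position as a lerp start.
; Tick slides all tiles back over one second, then destroys the oldest tiles and refreshes the cache.
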(event `self.ReceiveBeginPlay`
  (`self.SpawnTileSet` (`self.Length`)))

(event `self.ReceiveTick`
  (params (DeltaSeconds :type "Float (single-precision)"))
  (`self.MovingTiles`
    (:`then`
      (set `self.Moving Time` (+ DeltaSeconds (`self.Moving Time`)))
      (for _array_element (`self.All Tiles`)
        (bind _value (`BlueprintMapLibrary.Map_Find` (`self.Positions`) _array_element))
        (`self.K2_SetActorLocation` _array_element (`KismetMathLibrary.VLerp` _value (- _value (`KismetMathLibrary.MakeVector` (* (`self.Tile Size X`) (`self.Num Per Row`)))) (`self.Moving Time`)) false false))
      (if (>= (`self.Moving Time`) 1.0)
        (set `self.MovingTiles` false)
        (`self.Despawn Last Set`)
        (`self.Cache Tile Positions`)))
    (:`else`)))

(event `Move Tile Set`
  (`self.SpawnTileSet` 1)
  (`BlueprintMapLibrary.Map_Clear` (`self.Positions`))
  (`self.Cache Tile Positions`)
  (`KismetSystemLibrary.DelayUntilNextTick`)
  (set `self.MovingTiles` true)
  (set `self.Moving Time` 0.0))

(fn `Cache Tile Positions`
  (for _array_element (`self.All Tiles`)
    (`BlueprintMapLibrary.Map_Add` (`self.Positions`) _array_element (`self.K2_GetActorLocation` _array_element))))

(fn `Despawn Last Set`
  (bind (_arrayindex _arrayelement) (`/Engine/EditorBlueprintResources/StandardMacros.ReverseForEachLoop` (`self.All Tiles`))
    (:`LoopBody`
      (if (<= _arrayindex (* (- (`self.Num Per Row`) 1) (`self.Length`)))
        (`BlueprintMapLibrary.Map_Remove` (`self.Positions`) _arrayelement)
        (`self.K2_DestroyActor` _arrayelement)
        (`KismetArrayLibrary.Array_Remove` (`self.All Tiles`) _arrayindex)))))

(fn `Get Uppermost X Pos`
  (returns (X :type "Float (double-precision)"))
  (locals (`Highest Value` :type "Float (double-precision)" :default -9999999999.0) (Found :type Boolean))
  (bind (_keypin _valuepin) (`|MapForEach` (`self.Positions`))
    (:`then`
      (bind _x (.x _valuepin))
      (if (>= _x (`local.Highest Value`))
        (set `local.Highest Value` _x)
        (set `local.Found` true)))
    (:`CompletedPin`
      (return (`KismetMathLibrary.SelectFloat` (`local.Highest Value`) 0.0 (`local.Found`))))))

(fn `SpawnTileSet`
  (params (Length :type Integer :default 0))
  (locals (`Highest X` :type "Float (double-precision)" :default 0.0))
  (bind _highest_x (`local.Highest X`))
  (bind _highest_x_2 (`local.Highest X`))
  (bind _returnvalue (- (`self.Num Per Row`) 1))
  (set `local.Highest X` (`self.Get Uppermost X Pos`))
  (`KismetSystemLibrary.PrintString` (`KismetStringLibrary.Concat_StrStr` "OFFSET X: " (`KismetStringLibrary.Conv_DoubleToString` (`KismetMathLibrary.SelectFloat` 0.0 (+ (`self.Tile Size X`) _highest_x) (== _highest_x 0.0)))))
  (for _index (range (* Length (`self.Num Per Row`)))
    (for _index_2 (range (+ _returnvalue 1))
      (bind _returnvalue_2 (`|SpawnActorFromClass` "/Script/Engine.StaticMeshActor" (`KismetMathLibrary.MakeTransform` (`KismetMathLibrary.MakeVector` (+ (* _index (`self.Tile Size X`)) (`KismetMathLibrary.SelectFloat` 0.0 (+ (`self.Tile Size X`) _highest_x_2) (== _highest_x_2 0.0))) (+ (* _index_2 (`self.Tile Size Y`)) (/ (* _returnvalue (`self.Tile Size Y`) -1.0) 2.0) (`KismetMathLibrary.SelectFloat` 0.0 100.0 (== (mod _index 2) 0))) 50.0) (struct :`Yaw` 90.0) (`KismetMathLibrary.MakeVector` 100.0 100.0 200.0)) "AlwaysSpawn" "MultiplyWithRoot" self null))
      (`StaticMeshActor.SetMobility` _returnvalue_2 "Movable")
      (`StaticMeshComponent.SetStaticMesh` (`StaticMeshActor.StaticMeshComponent` _returnvalue_2) "/Game/Environment/tiles/hex_grass.hex_grass")
      (`KismetArrayLibrary.Array_Add` (`self.All Tiles`) _returnvalue_2)))
  (`self.Cache Tile Positions`))

(fn `UserConstructionScript`)
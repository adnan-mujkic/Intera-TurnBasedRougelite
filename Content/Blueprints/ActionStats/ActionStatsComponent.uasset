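; ActionStatsComponent holds a map of game stats and changes them through data-driven game effects.
; BeginPlay seeds the map from DefaultGameStats, and GetStatValue looks up a stat, returning zero if it is absent.
; ApplyGameEffect constructs an effect object from the passed class and applies each of its mods in order as Add, Multiply or Override.
; Results are written straight into the map, with no tracking or removal of applied effects.
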(event `self.ReceiveBeginPlay`
  (set `self.GameStats` (`self.DefaultGameStats`)))

(fn `ApplyGameEffect`
  (params (NewParam :type "/Game/Blueprints/ActionStats/GameEffect Class Reference"))
  (locals (GameEffect :type "/Game/Blueprints/ActionStats/GameEffect Object Reference"))
  (bind _gamestats (`self.GameStats`))
  (bind _returnvalue (`|GenericCreateObject` NewParam))
  (bind _output_get (set `local.GameEffect` _returnvalue))
  (for _array_element (`/Game/Blueprints/ActionStats/GameEffect.Mods` _output_get)
    (bind (_stattype _modoperation _value) (break `/Game/Blueprints/ActionStats/EffectMod` _array_element))
    (switch `/Game/Blueprints/ActionStats/ModOperation` _modoperation
      (:`NewEnumerator0`
        (bind _value_2 (`self.GetStatValue` _stattype))
        (`BlueprintMapLibrary.Map_Add` _gamestats _stattype (+ _value _value_2)))
      (:`NewEnumerator1`
        (`BlueprintMapLibrary.Map_Add` _gamestats _stattype (* _value_2 _value)))
      (:`NewEnumerator2`
        (`BlueprintMapLibrary.Map_Add` _gamestats _stattype _value)))))

(fn `GetStatValue`
  (params (Prima :type "/Game/Blueprints/ActionStats/StatType Enum" :default "NewEnumerator0"))
  (returns (Value :type "Float (double-precision)"))
  (bind (_value _returnvalue) (`BlueprintMapLibrary.Map_Find` (`self.GameStats`) Prima))
  (if _returnvalue
    (return _value)
    (else
      (return 0.0))))
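; ActorHoverComponent detects the BaseActor under the mouse cursor and shows its health in the player's stat widget.
; Each Tick it runs a complex cursor trace against WorldDynamic objects and sets any BaseActor hit as BP_MainPlayerController's currently hovered character.
; It passes that actor's current and max health from its ActionStatsComponent to the controller's StatWidget, cached on first use.
; A miss leaves the hovered character and widget unchanged.
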(event `self.ReceiveTick`
  (params (DeltaSeconds :type "Float (single-precision)"))
  (bind (_hitresult _returnvalue) (`PlayerController.GetHitResultUnderCursorForObjects` (`GameplayStatics.GetPlayerController` 0) (`|MakeArray` "ObjectTypeQuery2" :!type "EObjectTypeQuery Enum") true))
  (if _returnvalue
    (bind _asbase_actor (cast `/Game/Blueprints/Characters/BaseActor` (`.HitActor` (`GameplayStatics.BreakHitResult` _hitresult))))
    (bind _asbp_main_player_controller (cast `/Game/Blueprints/BP_MainPlayerController` (`GameplayStatics.GetPlayerController` 0)))
    (`/Game/Blueprints/BP_MainPlayerController.Set Currently Hovered Character` _asbp_main_player_controller _asbase_actor)
    (bind _statwidget (`self.Get Stat Widget`))
    (bind _actionstatscomponent (`/Game/Blueprints/Characters/BaseActor.ActionStatsComponent` _asbase_actor))
    (`/Game/UI/BP_UI/WBP_StatWidget.UpdateHealth` _statwidget (`/Game/Blueprints/ActionStats/ActionStatsComponent.GetStatValue` _actionstatscomponent "NewEnumerator0") (`/Game/Blueprints/ActionStats/ActionStatsComponent.GetStatValue` _actionstatscomponent "NewEnumerator1"))))

(fn `Get Stat Widget`
  (returns (StatWidget :type "/Game/UI/BP_UI/WBP_StatWidget Object Reference"))
  (`self.Cached Stat Widget`
    (:`then`
      _)
    (:`else`
      (bind _asbp_main_player_controller (cast `/Game/Blueprints/BP_MainPlayerController` (`GameplayStatics.GetPlayerController` 0)))
      (set `self.Cached Stat Widget` (`/Game/Blueprints/BP_MainPlayerController.StatWidget` _asbp_main_player_controller))))
  (return (`self.Cached Stat Widget`)))
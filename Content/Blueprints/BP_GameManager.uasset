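; Game manager for turn-based one-on-one combat between the player's Barbarian and a spawned enemy.
; StartTurn checks win/lose and alternates sides by turn-counter parity, filling the action widget for the player or auto-casting the enemy's first ability after a delay.
; A win moves the level generator's tile set and starts a new round with a fresh enemy.
; A loss destroys both combatants and shows the lose screen.
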(fn `CheckWinLose`
  (if (<= (`/Game/Blueprints/ActionStats/ActionStatsComponent.GetStatValue` (`/Game/Blueprints/Characters/BaseActor.ActionStatsComponent` (`self.Barbarian`)) "NewEnumerator0") 0.0)
    (`self.GameLose`)
    (elif (<= (`/Game/Blueprints/ActionStats/ActionStatsComponent.GetStatValue` (`/Game/Blueprints/Characters/BaseActor.ActionStatsComponent` (`self.Enemy`)) "NewEnumerator0") 0.0)
      (`self.GameWin`))))

(fn `GameLose`
  (`self.K2_DestroyActor` (`self.Enemy`))
  (`self.K2_DestroyActor` (`self.Barbarian`))
  (set `self.GameRunning` false)
  (bind _asbp_main_player_controller (cast `/Game/Blueprints/BP_MainPlayerController` (`GameplayStatics.GetPlayerController` 0)))
  (`/Game/UI/BP_UI/WBP_MainMenu.Show Lose Screen` (`/Game/Blueprints/BP_MainPlayerController.MainWidget` _asbp_main_player_controller)))

(fn `GameStart`
  (set `self.GameRunning` true)
  (`self.SpawnHeros`)
  (`self.SpawnEnemies`)
  (bind _returnvalue (`|CreateWidget` "/Game/UI/BP_UI/WBP_ActionWidget.WBP_ActionWidget_C"))
  (bind _output_get (set `self.ActionWidget` _returnvalue))
  (`UserWidget.AddToViewport` _output_get 0)
  (`self.StartTurn`))

(fn `GameWin`
  (set `self.GameRunning` false)
  (bind _returnvalue (`GameplayStatics.GetActorOfClass` "/Game/Blueprints/BP_LevelGenerationManager.BP_LevelGenerationManager_C"))
  (`/Game/Blueprints/BP_LevelGenerationManager.Move Tile Set` _returnvalue)
  (`self.K2_DestroyActor` (`self.Enemy`))
  (`KismetSystemLibrary.K2_SetTimer` null "Start New Round" 1.1))

(fn `GetCaster`
  (returns (Caster :type "/Game/Blueprints/Characters/BaseActor Object Reference"))
  (if (`self.PlayerTurn`)
    (return (`self.Barbarian`))
    (else
      (return (`self.Enemy`)))))

(fn `GetTarget`
  (returns (Target :type "/Game/Blueprints/Characters/BaseActor Object Reference"))
  (if (`self.PlayerTurn`)
    (return (`self.Enemy`))
    (else
      (return (`self.Barbarian`)))))

(fn `ProcessEnemyTurn`
  (bind _caster (`self.GetCaster`))
  (bind _actionstatscomponent (`/Game/Blueprints/Characters/BaseActor.ActionStatsComponent` _caster))
  (`KismetSystemLibrary.PrintString` "ENEMY TURN!!1!")
  (`/Game/Blueprints/ActionStats/ActionStatsComponent.ActivateAbility` _actionstatscomponent (`|GetArrayItem` (`/Game/Blueprints/ActionStats/ActionStatsComponent.AbilityList` _actionstatscomponent)) _caster (`self.GetTarget`))
  (`self.StartTurn`))

(fn `SpawnEnemies`
  (bind _returnvalue (`|SpawnActorFromClass` "/Game/Blueprints/Characters/BP_Enemy.BP_Enemy_C" (`KismetMathLibrary.MakeTransform` (360.0 0.0 50.0) (struct :`Yaw` 90.0)) "Undefined" "MultiplyWithRoot" null null))
  (set `self.Enemy` _returnvalue))

(fn `SpawnHeros`
  (bind _returnvalue (`|SpawnActorFromClass` "/Game/Blueprints/Characters/BP_Barbarian.BP_Barbarian_C" (`KismetMathLibrary.MakeTransform` (0.0 0.0 50.0) (struct :`Yaw` -90.0)) "Undefined" "MultiplyWithRoot" null null))
  (set `self.Barbarian` _returnvalue))

(fn `Start New Round`
  (set `self.GameRunning` true)
  (`self.SpawnEnemies`)
  (set `self.TurnNumber` 0)
  (`self.StartTurn`))

(fn `StartTurn`
  (`self.CheckWinLose`)
  (`self.GameRunning`
    (:`then`
      (bind _result (`/Engine/EditorBlueprintResources/StandardMacros.IncrementInt` (`self.TurnNumber`))
        (:`  `
          (bind _output_get (set `self.PlayerTurn` (!= (mod _result 2) 0)))
          (`Widget.SetVisibility` (`self.ActionWidget`) (select `bool` _output_get :`false` "Hidden" :`true` "Visible" :!type "ESlateVisibility Enum"))
          (if (`self.PlayerTurn`)
            (`/Game/UI/BP_UI/WBP_ActionWidget.PopulateAbilities` (`self.ActionWidget`) (`/Game/Blueprints/ActionStats/ActionStatsComponent.AbilityList` (`/Game/Blueprints/Characters/BaseActor.ActionStatsComponent` (`self.GetCaster`))))
            (else
              (`KismetSystemLibrary.K2_SetTimer` null "ProcessEnemyTurn" 1.0 false true))))))
    (:`else`)))

(fn `UserConstructionScript`)
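; BP_BaseAttackAbility is an attack ability that applies a stat-scaled game effect from a caster to a target.
; Activate constructs the first GameEffects entry and overwrites its first mod's value with a caster stat times BaseDamage, negated so damage acts as a reduction.
; The modified effect instance is then applied through the target's ActionStatsComponent.
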(fn `Activate`
  (params (Caster :type "/Game/Blueprints/Characters/BaseActor Object Reference") (Target :type "/Game/Blueprints/Characters/BaseActor Object Reference"))
  (locals (LocalEffect :type "/Game/Blueprints/ActionStats/GameEffect Object Reference"))
  (bind _returnvalue (`|GenericCreateObject` (`|GetArrayItem` (`self.GameEffects`))))
  (bind _output_get (set `local.LocalEffect` _returnvalue))
  (bind _mods (`/Game/Blueprints/ActionStats/GameEffect.Mods` _output_get))
  (bind _structout (setmembers `/Game/Blueprints/ActionStats/EffectMod` :`StructRef` (`|GetArrayItem` _mods) :`Value` (* (`/Game/Blueprints/ActionStats/ActionStatsComponent.GetStatValue` (`/Game/Blueprints/Characters/BaseActor.ActionStatsComponent` Caster) "NewEnumerator2") (`self.BaseDamage`) -1.0)))
  (`KismetArrayLibrary.Array_Set` _mods 0 _structout)
  (`/Game/Blueprints/ActionStats/ActionStatsComponent.ApplyGameEffectObject` (`/Game/Blueprints/Characters/BaseActor.ActionStatsComponent` Target) (`local.LocalEffect`)))